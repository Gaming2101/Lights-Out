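; BP_Light is a short-lived coloured light actor that removes itself on a timer or when the player comes near.
; On BeginPlay it sets the light colour and a dynamic material's Colour parameter on Object, using separate random picks from Colours, so the two can differ.
; It destroys itself after a random delay of a few seconds, or sooner if Tick finds the player pawn within a fixed distance.
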(event `self.ReceiveBeginPlay`
  (bind _outitem (`KismetArrayLibrary.Array_Random` (`self.Colours`)))
  ;[1 1 1] Controls the colour of the light
  (`LightComponent.SetLightColor` (`self.Light`) _outitem true)
  (bind _returnvalue (`PrimitiveComponent.CreateDynamicMaterialInstance` (`self.Object`) 0 "/Game/Materials/Light_Mat.Light_Mat" "None"))
  (`MaterialInstanceDynamic.SetVectorParameterValue` _returnvalue "Colour" _outitem)
  (`KismetSystemLibrary.Delay` (`KismetMathLibrary.RandomFloatInRange` 3.0 7.0))
  (`self.K2_DestroyActor`))

(event `self.ReceiveTick`
  (params (DeltaSeconds :type "Float (single-precision)"))
  ;[1 1 1] Destroys the light if the player gets too close
  (if (< (`self.GetDistanceTo` (`GameplayStatics.GetPlayerPawn` 0)) 1550.0)
    (`self.K2_DestroyActor`)))

(fn `UserConstructionScript`)