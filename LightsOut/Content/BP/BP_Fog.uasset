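; BP_Fog is an actor that displays fog with adjustable size and opacity.
; The construction script scales the root uniformly by Radius and creates a dynamic material instance from Fog_Mat on the Fog component, setting its Opacity from Intensity.
; Tick reapplies both values every frame, so runtime changes to Radius or Intensity show immediately.
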(event `self.ReceiveTick`
  (params (DeltaSeconds :type "Float (single-precision)"))
  ;[1 1 1] Controls the size and opacity of the fog
  (`SceneComponent.SetRelativeScale3D` (`self.DefaultSceneRoot`) (`KismetMathLibrary.Conv_DoubleToVector` (`self.Radius`)))
  (`MaterialInstanceDynamic.SetScalarParameterValue` (`self.Fog_Dynamic`) "Opacity" (`self.Intensity`)))

(fn `UserConstructionScript`
  ;[1 1 1] Controls the size and opacity of the fog
  (`SceneComponent.SetRelativeScale3D` (`self.DefaultSceneRoot`) (`KismetMathLibrary.Conv_DoubleToVector` (`self.Radius`)))
  (bind _returnvalue (`PrimitiveComponent.CreateDynamicMaterialInstance` (`self.Fog`) 0 "/Game/Materials/Fog_Mat.Fog_Mat" "None"))
  (set `self.Fog_Dynamic` _returnvalue)
  (`MaterialInstanceDynamic.SetScalarParameterValue` (`self.Fog_Dynamic`) "Opacity" (`self.Intensity`)))