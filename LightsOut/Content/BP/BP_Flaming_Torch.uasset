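; Flaming torch actor that can be lit, burns out on a random timer and reports to the Game_HUD actor's lit-torch count.
; It starts lit on BeginPlay; LightFlame relights it and, once the game has started, extinguishes it after a delay scaled from AverageBurnTime.
; SetUp switches particles, light and sound on or off, using staggered delays and particle time dilation to speed up flame transitions.
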(event `self.ReceiveBeginPlay`
  ;[1 1 1] Sets up the variables
  (bind _returnvalue (`GameplayStatics.GetActorOfClass` "/Game/FirstPerson/Systems/Game_HUD.Game_HUD_C"))
  (set `self.GameHud` _returnvalue)
  (set `self.Active` true)
  (`self.Set Up`))

(event `Light Flame`
  (bind _average_burn_time (`/Game/FirstPerson/Systems/Game_HUD.Average Burn Time` (`self.GameHud`)))
  ;[1 1 1] Lights the Flame, and then stops it after some time
  (set `self.Active` true)
  (`self.Set Up`)
  (if (`/Game/FirstPerson/Systems/Game_HUD.Started` (`self.GameHud`))
    (`KismetSystemLibrary.Delay` (`KismetMathLibrary.RandomFloatInRange` (/ _average_burn_time 2.0) (* _average_burn_time 2.0)))
    (set `self.Active` false)
    (`self.Set Up`)))

(event `Set Up`
  (bind _gamehud (`self.GameHud`))
  (bind _gamehud_2 (`self.GameHud`))
  (bind _flaming_torch_sfx (`self.Flaming_Torch_SFX`))
  (bind _light (`self.Light`))
  (bind _p_fire_torch (`self.P_Fire_Torch`))
  ;[1 1 1] Controls the fire, light and sound when setting up the flame
  (if (`self.Active`)
    (`ParticleSystemComponent.BeginTrails` _p_fire_torch "None" "None" "ETrailWidthMode_FromCentre" 0.0)
    (if (`/Game/FirstPerson/Systems/Game_HUD.Started` _gamehud_2)
      (`GameplayStatics.PlaySoundAtLocation` "/Game/SFX/Flaming_Torch_Lit_SFX.Flaming_Torch_Lit_SFX" (`SceneComponent.K2_GetComponentLocation` (`self.Light`)) (struct) 3.0 1.0 0.0 null null null null))
    (set `ParticleSystemComponent.CustomTimeDilation` 5.0 _p_fire_torch)
    (`KismetSystemLibrary.Delay` 0.35)
    (set `ParticleSystemComponent.CustomTimeDilation` 1.0 _p_fire_torch)
    (`KismetSystemLibrary.Delay` 0.2)
    (`SceneComponent.SetVisibility` _light true false)
    (`KismetSystemLibrary.Delay` 0.9)
    (`AudioComponent.Play` _flaming_torch_sfx 0.0)
    (set `/Game/FirstPerson/Systems/Game_HUD.Amount Of Torches Lit` (+ (`/Game/FirstPerson/Systems/Game_HUD.Amount Of Torches Lit` _gamehud) 1) _gamehud)
    (else
      (`ParticleSystemComponent.EndTrails` _p_fire_torch)
      (set `ParticleSystemComponent.CustomTimeDilation` 5.0 _p_fire_torch)
      (`SceneComponent.SetVisibility` _light false false)
      (`AudioComponent.Stop` _flaming_torch_sfx)
      (set `/Game/FirstPerson/Systems/Game_HUD.Amount Of Torches Lit` (- (`/Game/FirstPerson/Systems/Game_HUD.Amount Of Torches Lit` _gamehud_2) 1) _gamehud_2))))

(fn `UserConstructionScript`)