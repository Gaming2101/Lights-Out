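; BP_Monster is a short-lived monster actor that turns to face the player and vanishes when approached.
; Every tick it rotates toward the player pawn and destroys itself within a fixed distance.
; A recently-rendered check adds a delayed destroy at the same range, but the unconditional distance check makes it redundant.
; A delay started on BeginPlay also removes it after a few seconds.
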(event `self.ReceiveBeginPlay`
  ;[1 1 1] Destroys the monster after a certain time
  (`KismetSystemLibrary.Delay` 8.0)
  (`self.K2_DestroyActor`))

(event `self.ReceiveTick`
  (params (DeltaSeconds :type "Float (single-precision)"))
  ;[1 1 1] Makes the monster face the player, and aslo destroys it if the player gets too close or looks at it
  (`self.K2_SetActorRotation` (`KismetMathLibrary.FindLookAtRotation` (`self.K2_GetActorLocation`) (`self.K2_GetActorLocation` (`GameplayStatics.GetPlayerPawn` 0))))
  (`|ExecutionSequence`
    (:`then_0`
      (if (and (`self.WasRecentlyRendered` 0.1) (< (`self.GetDistanceTo` (`GameplayStatics.GetPlayerPawn` 0)) 400.0))
        (`KismetSystemLibrary.Delay` 0.001)
        (`self.K2_DestroyActor`)))
    (:`then_1`
      (if (< (`self.GetDistanceTo` (`GameplayStatics.GetPlayerPawn` 0)) 400.0)
        (`self.K2_DestroyActor`)))))

(fn `UserConstructionScript`)